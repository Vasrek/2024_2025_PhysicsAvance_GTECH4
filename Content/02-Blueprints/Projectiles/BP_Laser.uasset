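; BP_Laser is a short-lived laser projectile that triggers a master field when it hits objects tagged "GC".
; On such a capsule overlap it spawns a scaled-up BP_MyMasterField at its location, sets the activation type and fires CETrigger.
; After a brief delay it destroys both the field and itself.
; Any other overlap destroys the laser immediately, and a lifespan set at BeginPlay removes it otherwise.
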(event `self.ReceiveBeginPlay`
  (`self.SetLifeSpan` 5.0))

(event `self.Capsule.OnComponentBeginOverlap`
  (params (OverlappedComponent :type "PrimitiveComponent Object Reference") (OtherActor :type "Actor Object Reference") (OtherComp :type "PrimitiveComponent Object Reference") (OtherBodyIndex :type Integer) (bFromSweep :type Boolean) (SweepResult :type "HitResult Structure (by ref)"))
  (if (`self.ActorHasTag` OtherActor "GC")
    (bind _returnvalue (`|SpawnActorFromClass` "/Game/02-Blueprints/Force/BP_MyMasterField.BP_MyMasterField_C" (`KismetMathLibrary.MakeTransform` (`self.K2_GetActorLocation`) (struct) (5.0 5.0 5.0)) "Undefined" "MultiplyWithRoot" null null))
    (set `/Engine/EditorResources/FieldNodes/FS_MasterField.ActivationType` "NewEnumerator4" _returnvalue)
    (`/Engine/EditorResources/FieldNodes/FS_MasterField.CE_Trigger` _returnvalue)
    (`KismetSystemLibrary.Delay` 0.2)
    (`self.K2_DestroyActor` _returnvalue)
    (`self.K2_DestroyActor` self)
    (else
      (`self.K2_DestroyActor`))))

(fn `UserConstructionScript`)