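; BP_Hover is a player-controlled hover vehicle driven by Enhanced Input, adding its mapping context on BeginPlay.
; Thrust and steer inputs set target linear and angular speeds on BPMovementComponent, with boost held to multiply thrust.
; Flip rights the vehicle when it is on its side or upside down, using an impulse along its negative up vector, then a delayed roll impulse.
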(event `self.ReceiveBeginPlay`
  (bind _returnvalue (pcsubsystem `EnhancedInputLocalPlayerSubsystem` (`GameplayStatics.GetPlayerController` 0)))
  (`/Engine/EditorBlueprintResources/StandardMacros.IsValid` _returnvalue
    (:`Is Valid`
      (`EnhancedInputSubsystemInterface.AddMappingContext` _returnvalue "/Game/02-Blueprints/Inputs/IMC_Hover.IMC_Hover" 0 (struct)))))

(event `EnhancedInput|/Game/02-Blueprints/Inputs/Actions/IA_Thrust`
  (params (ActionValue :type "Float (double-precision)") (ElapsedSeconds :type "Float (double-precision)") (TriggeredSeconds :type "Float (double-precision)") (InputAction :type "InputAction Object Reference" :default "/Game/02-Blueprints/Inputs/Actions/IA_Thrust.IA_Thrust"))
  (bind _bp_movementcomponent (`self.BP_MovementComponent`))
  (:`Triggered`
    (set `/Game/02-Blueprints/Hover/BP_MovementComponent.TargetSpeed` (* ActionValue (`self.ThurstSpeed`) (`self.BoostMultiplier`)) _bp_movementcomponent))
  (:`Completed`
    (set `/Game/02-Blueprints/Hover/BP_MovementComponent.TargetSpeed` 0.0 _bp_movementcomponent)))

(event `EnhancedInput|/Game/02-Blueprints/Inputs/Actions/IA_Steer`
  (params (ActionValue :type "Float (double-precision)") (ElapsedSeconds :type "Float (double-precision)") (TriggeredSeconds :type "Float (double-precision)") (InputAction :type "InputAction Object Reference" :default "/Game/02-Blueprints/Inputs/Actions/IA_Steer.IA_Steer"))
  (bind _bp_movementcomponent (`self.BP_MovementComponent`))
  (:`Triggered`
    (set `/Game/02-Blueprints/Hover/BP_MovementComponent.TargetAngularSpeed` (* ActionValue (`self.AngularRotSpeed`)) _bp_movementcomponent))
  (:`Completed`
    (set `/Game/02-Blueprints/Hover/BP_MovementComponent.TargetAngularSpeed` 0.0 _bp_movementcomponent)))

(event `EnhancedInput|/Game/02-Blueprints/Inputs/Actions/IA_Boost`
  (params (ActionValue :type Boolean) (ElapsedSeconds :type "Float (double-precision)") (TriggeredSeconds :type "Float (double-precision)") (InputAction :type "InputAction Object Reference" :default "/Game/02-Blueprints/Inputs/Actions/IA_Boost.IA_Boost"))
  (:`Triggered`
    (set `self.BoostMultiplier` 3.0))
  (:`Completed`
    (set `self.BoostMultiplier` 1.0)))

(event `EnhancedInput|/Game/02-Blueprints/Inputs/Actions/IA_Flip`
  (params (ActionValue :type Boolean) (ElapsedSeconds :type "Float (double-precision)") (TriggeredSeconds :type "Float (double-precision)") (InputAction :type "InputAction Object Reference" :default "/Game/02-Blueprints/Inputs/Actions/IA_Flip.IA_Flip"))
  (bind _vehicle (`self.Vehicle`))
  (bind _vehicle_2 (`self.Vehicle`))
  (:`Started`
    (if (<= (`KismetMathLibrary.Dot_VectorVector` (`SceneComponent.GetUpVector` (`self.Vehicle`)) (`KismetMathLibrary.MakeVector` 0.0 0.0 1.0)) 0.2)
      (`PrimitiveComponent.AddImpulse` _vehicle (* (`SceneComponent.GetUpVector` _vehicle) -1000000.0) "None" false)
      (`KismetSystemLibrary.Delay` 0.2)
      (`PrimitiveComponent.AddAngularImpulseInDegrees` _vehicle_2 (* (`SceneComponent.GetForwardVector` _vehicle_2) 1000000000.0) "None" false))))

(fn `UserConstructionScript`)